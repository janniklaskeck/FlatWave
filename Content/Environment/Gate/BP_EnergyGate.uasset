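; BP_EnergyGate is a gate that starts sunk below its placed position and rises to close when activated.
; BeginPlay stores the placed position as closed and drops the actor by its full height.
; Activate enables Cube collision and lets Tick lerp it upward; Deactivate disables collision and halts movement without lowering it or resetting progress.
; The construction script scales the Cube from Extents.
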(event EventTick
  (params (DeltaSeconds :type Float%20%28single-precision%29))
  (|CallParentFunction DeltaSeconds)
  (if (Variables|Default|GetShouldClose)
    (bind _output_get (Variables|Default|SetMoveCounter (+ (Variables|Default|GetMoveCounter) (* DeltaSeconds (Variables|Default|GetMoveSpeed)))))
    (Transformation|SetActorLocation (Math|Vector|Lerp(Vector) (Variables|Default|GetOpenPosition) (Variables|Default|GetClosedPosition) (Math|Float|Clamp(Float) _output_get)) false false)))

(event EventActivate
  (Collision|SetCollisionEnabled (Variables|Default|GetCube) "QueryAndPhysics")
  (Variables|Default|SetShouldClose true))

(event EventDeactivate
  (Collision|SetCollisionEnabled (Variables|Default|GetCube) "NoCollision")
  (Variables|Default|SetShouldClose false))

(event EventBeginPlay
  (bind _returnvalue (Transformation|GetActorLocation))
  (|CallParentFunction)
  (Variables|Default|SetClosedPosition _returnvalue)
  (bind _output_get (Variables|Default|SetOpenPosition (- _returnvalue (Math|Vector|MakeVector 0.0 0.0 (* (.z (Variables|Default|GetExtents)) 2.0)))))
  (Transformation|SetActorLocation _output_get false false))

(fn ConstructionScript
  (Transformation|SetWorldScale3D (Variables|Default|GetCube) (/ (Variables|Default|GetExtents) 5e+01)))