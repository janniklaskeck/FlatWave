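; BP_DirectionArrows is an environment Blueprint with three direction arrows that light up in an active color.
; On BeginPlay it creates one dynamic material instance from the first arrow's material, shares it across all three, and sets its emissive color to dim gray.
; The Activate event switches that shared emissive color to ActiveColor, and BeginPlay calls it immediately when ActivateOnBeginPlay is set.
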(event EventActivate
  (Rendering|Material|SetVectorParameterValue (Variables|Default|GetArrowMaterialInstance) "EmissiveColor" (Variables|Default|GetActiveColor) :!class /Script/Engine.MaterialInstanceDynamic))

(event EventBeginPlay
  (bind _arrow1 (Variables|Default|GetArrow1))
  (|CallParentFunction)
  (bind _returnvalue (Rendering|Material|CreateDynamicMaterialInstance _arrow1 0 (Rendering|Material|GetMaterial _arrow1 0) "None" :!class /Script/Engine.PrimitiveComponent))
  (bind _output_get (Variables|Default|SetArrowMaterialInstance _returnvalue))
  (Rendering|Material|SetMaterial (Variables|Default|GetArrow1) 0 _output_get)
  (Rendering|Material|SetVectorParameterValue (Variables|Default|GetArrowMaterialInstance) "EmissiveColor" "(R=0.305882,G=0.305882,B=0.305882,A=0.000000)" :!class /Script/Engine.MaterialInstanceDynamic)
  (if (Variables|Default|GetActivateOnBeginPlay)
    (Class|FWScenarioGate|Activate)))

(fn ConstructionScript)