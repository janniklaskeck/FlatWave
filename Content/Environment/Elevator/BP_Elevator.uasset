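; BP_Elevator is a lift volume that pushes player characters upward while active, sized in the construction script from Extent.
; Entering the box saves the character's gravity scale in one shared variable and zeroes it, and exiting restores it.
; Tick applies a vertical Force to every overlapping player's CharacterMovement.
; Activate and Deactivate toggle IsActive and the particles; gravity changes only on overlaps while active, so deactivation does not restore it.
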(event OnComponentBeginOverlap(Box)
  (params (OverlappedComponent :type Primitive%20Component%20Object%20Reference) (OtherActor :type Actor%20Object%20Reference) (OtherComp :type Primitive%20Component%20Object%20Reference) (OtherBodyIndex :type Integer) (bFromSweep :type Boolean) (SweepResult :type Hit%20Result%20Structure%20%28by%20ref%29))
  (if (Variables|Default|GetIsActive)
    (bind _asfwplayer_character_base (Utilities|Casting|CastToFWPlayerCharacterBase OtherActor))
    (Variables|Default|SetPreviousGravityScale (Variables|/Script/Engine.CharacterMovementComponent|GetGravityScale (Variables|/Script/Engine.Character|GetCharacterMovement _asfwplayer_character_base)))
    (Variables|/Script/Engine.CharacterMovementComponent|SetGravityScale (Variables|/Script/Engine.Character|GetCharacterMovement _asfwplayer_character_base) 0.0)))

(event OnComponentEndOverlap(Box)
  (params (OverlappedComponent :type Primitive%20Component%20Object%20Reference) (OtherActor :type Actor%20Object%20Reference) (OtherComp :type Primitive%20Component%20Object%20Reference) (OtherBodyIndex :type Integer))
  (if (Variables|Default|GetIsActive)
    (bind _asfwplayer_character_base (Utilities|Casting|CastToFWPlayerCharacterBase OtherActor))
    (Variables|/Script/Engine.CharacterMovementComponent|SetGravityScale (Variables|/Script/Engine.Character|GetCharacterMovement _asfwplayer_character_base) (Variables|Default|GetPreviousGravityScale))))

(event EventDeactivate
  (Components|Activation|Deactivate (Variables|Default|GetParticleSystem))
  (Variables|Default|SetIsActive false))

(event EventActivate
  (Components|Activation|Activate (Variables|Default|GetParticleSystem) false)
  (Variables|Default|SetIsActive true))

(event EventTick
  (params (DeltaSeconds :type Float%20%28single-precision%29))
  (if (Variables|Default|GetIsActive)
    (for _array_element (Collision|GetOverlappingActors (Variables|Default|GetBox) "/Script/FlatWave.FWPlayerCharacterBase" :!class /Script/Engine.PrimitiveComponent)
      (bind _asfwplayer_character_base (Utilities|Casting|CastToFWPlayerCharacterBase _array_element))
      (Physics|AddForce (Variables|/Script/Engine.Character|GetCharacterMovement _asfwplayer_character_base) (Math|Vector|MakeVector 0.0 0.0 (Variables|Default|GetForce))))))

(fn ConstructionScript
  (Components|Box|SetBoxExtent (Variables|Default|GetBox) (Variables|Default|GetExtent) true))