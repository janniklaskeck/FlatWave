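; Resizable floor-and-walls geometry piece, built from FloorWidth, FloorLength and WallHeight.
; The construction script scales the Floor, then runs four sequence steps that scale WallX and WallY pieces and offset them to opposite floor edges.
; Offsets are 50 times each dimension, consistent with centered 100-unit meshes, with walls raised by half their height.
; The event graph has no active logic.
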(event EventBeginPlay)

(event Collision|EventActorBeginOverlap
  (params (OtherActor :type Actor%20Object%20Reference)))

(event EventTick
  (params (DeltaSeconds :type Float%20%28single-precision%29)))

(fn ConstructionScript
  (bind _wally_ (Variables|Default|GetWallY+))
  (bind _wally__2 (Variables|Default|GetWallY-))
  (bind _wallx_ (Variables|Default|GetWallX+))
  (bind _wallx__2 (Variables|Default|GetWallX-))
  (Transformation|SetWorldScale3D (Variables|Default|GetFloor) (Math|Vector|MakeVector (Variables|Default|GetFloorWidth) (Variables|Default|GetFloorLength) 1.0))
  (Utilities|FlowControl|Sequence
    (:then_0
      (Transformation|SetWorldScale3D _wallx__2 (Math|Vector|MakeVector 1.0 (Variables|Default|GetFloorLength) (Variables|Default|GetWallHeight)))
      (Transformation|SetRelativeLocation _wallx__2 (Math|Vector|MakeVector (* (Variables|Default|GetFloorWidth) -5e+01) 0.0 (* (Variables|Default|GetWallHeight) 5e+01)) false false))
    (:then_1
      (Transformation|SetWorldScale3D _wallx_ (Math|Vector|MakeVector 1.0 (Variables|Default|GetFloorLength) (Variables|Default|GetWallHeight)))
      (Transformation|SetRelativeLocation _wallx_ (Math|Vector|MakeVector (* (Variables|Default|GetFloorWidth) 5e+01) 0.0 (* (Variables|Default|GetWallHeight) 5e+01)) false false))
    (:then_2
      (Transformation|SetWorldScale3D _wally__2 (Math|Vector|MakeVector (Variables|Default|GetFloorWidth) 1.0 (Variables|Default|GetWallHeight)))
      (Transformation|SetRelativeLocation _wally__2 (Math|Vector|MakeVector 0.0 (* (Variables|Default|GetFloorLength) -5e+01) (* (Variables|Default|GetWallHeight) 5e+01)) false false))
    (:then_3
      (Transformation|SetWorldScale3D _wally_ (Math|Vector|MakeVector (Variables|Default|GetFloorWidth) 1.0 (Variables|Default|GetWallHeight)))
      (Transformation|SetRelativeLocation _wally_ (Math|Vector|MakeVector 0.0 (* (Variables|Default|GetFloorLength) 5e+01) (* (Variables|Default|GetWallHeight) 5e+01)) false false))))