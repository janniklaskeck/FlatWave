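; BP_MainGameMode is the main game mode Blueprint, which manages the game's background music.
; On BeginPlay it creates a 2D sound from Cue_GameMusic, stores it in GameMusic and plays it from the start.
; When destroyed, it stops the music if that audio component is still valid.
; Tick only calls the parent, and the construction script is empty.
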(event EventTick
  (params (DeltaSeconds :type Float%20%28single-precision%29))
  (|CallParentFunction DeltaSeconds))

(event EventBeginPlay
  (|CallParentFunction)
  (bind _returnvalue (Audio|CreateSound2D "/Game/Audio/Music/Cue_GameMusic.Cue_GameMusic" 1.0 1.0 0.0 0))
  (bind _output_get (Variables|Default|SetGameMusic _returnvalue))
  (Audio|Components|Audio|Play _output_get 0.0))

(event EventDestroyed
  (bind _gamemusic (Variables|Default|GetGameMusic))
  (|CallParentFunction)
  (Utilities|IsValid _gamemusic
    (:Is%20Valid
      (Audio|Components|Audio|Stop _gamemusic))))

(fn ConstructionScript)