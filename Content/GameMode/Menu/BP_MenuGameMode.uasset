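; BP_MenuGameMode is the game mode for the main menu, setting up its UI and music.
; On BeginPlay it creates W_MainMenu, adds it to the viewport and switches to UI-only input, focused on the start button with the mouse locked in fullscreen.
; It then plays Latin_Industries_Cue as a 2D sound stored in MenuMusic, which is stopped when the game mode is destroyed.
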(event EventBeginPlay
  (bind _returnvalue (UserInterface|CreateWidget "/Game/UI/MainMenu/W_MainMenu.W_MainMenu_C"))
  (UserInterface|Viewport|AddtoViewport _returnvalue 0)
  (Input|SetInputModeUIOnly (Game|GetPlayerController 0) (Variables|/Game/UI/MainMenu/W_MainMenu.W_MainMenu_C|GetStartGameButton _returnvalue) "LockInFullscreen")
  (bind _returnvalue_2 (Audio|CreateSound2D "/Game/Audio/Music/Latin_Industries_Cue.Latin_Industries_Cue" 1.0 1.0 0.0 0))
  (bind _output_get (Variables|Default|SetMenuMusic _returnvalue_2))
  (Audio|Components|Audio|Play _output_get 0.0))

(event EventTick
  (params (DeltaSeconds :type Float%20%28single-precision%29)))

(event EventDestroyed
  (Audio|Components|Audio|Stop (Variables|Default|GetMenuMusic)))

(fn ConstructionScript)